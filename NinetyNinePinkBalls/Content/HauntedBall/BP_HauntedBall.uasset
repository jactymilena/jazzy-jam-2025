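; BP_HauntedBall is an AI-controlled haunted ball character that reports its state relative to the player to its Blackboard.
; BeginPlay caches the first-person player next tick and gives the ball a small upward launch.
; Tick, throttled by a 0.2-second Delay, writes player distance, recent-render status, remaining jump-aways and Mood.
; A debug-drawn visibility trace from above the player's origin sets the line-of-sight key when unblocked.
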(event EventBeginPlay
  (Utilities|FlowControl|DelayUntilNextTick)
  (bind _asbp_first_person_character (Utilities|Casting|CastToBP_FirstPersonCharacter (Game|Player|GetPlayerPawn 0)))
  (Variables|Default|SetPlayer%20Reference _asbp_first_person_character)
  (Character|LaunchCharacter self "0.000000,0.000000,100.000000" false false))

(event EventTick
  (params (DeltaSeconds :type Float%20%28single-precision%29))
  (bind _returnvalue (Game|GetPlayerCharacter 0))
  (bind _self self)
  (bind _returnvalue_2 (Transformation|GetActorLocation _returnvalue))
  (bind _returnvalue_3 (AI|GetAIController _self))
  (bind _returnvalue_4 (AI|GetBlackboard _returnvalue_3))
  (Utilities|FlowControl|Delay 0.2)
  (AI|Components|Blackboard|SetValueasFloat _returnvalue_4 (Utilities|Name|MakeLiteralName "DistanceFromPlayer") (Math|Vector|Distance(Vector) (Transformation|GetActorLocation (Variables|Default|GetPlayer%20Reference)) (Transformation|GetActorLocation self)))
  (AI|Components|Blackboard|SetValueasBool _returnvalue_4 (Utilities|Name|MakeLiteralName "RecentlyRendered?") (Class|Actor|WasRecentlyRendered 0.2))
  (Class|BlackboardComponent|SetValueasInt _returnvalue_4 (Utilities|Name|MakeLiteralName "JumpAwayRemaining") (Variables|Default|GetJumpAway%20Remaining))
  (AI|Components|Blackboard|SetValueasEnum _returnvalue_4 (Utilities|Name|MakeLiteralName "Mood") (Variables|Default|GetMood))
  (bind _outhit (Collision|LineTraceByChannel (Math|Vector|MakeVector (.x _returnvalue_2) (.y _returnvalue_2) (+ (.z _returnvalue_2) 6e+01)) (Transformation|GetActorLocation) "TraceTypeQuery1" false 0 "ForDuration" true "(R=1.000000,G=0.000000,B=0.000000,A=1.000000)" "(R=0.000000,G=1.000000,B=0.000000,A=1.000000)" 0.6))
  (AI|Components|Blackboard|SetValueasBool _returnvalue_4 (Utilities|Name|MakeLiteralName "IsInLOSofPlayer?") (not (.bBlockingHit (Collision|BreakHitResult _outhit)))))

(fn ConstructionScript)